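; Short-lived Paper2D effect actor that shows a sprite for about two seconds, bracketed by flash effects on appearance and disappearance.
; On BeginPlay it plays a pitched-up Flash2 sound and spawns an enlarged Impulse_R at the sprite, then makes the sprite visible after a brief delay.
; After the hold it repeats the sound and impulse, then destroys itself shortly afterwards.
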(event EventBeginPlay
  ;[1 1 1] Begin Play
  (bind _returnvalue (Audio|SpawnSound2D "/Game/Se/Flash2.Flash2" 1.0 1.0 0.0 0))
  (Audio|Components|Audio|SetPitchMultiplier _returnvalue 1.2)
  (Audio|Components|Audio|SetVolumeMultiplier _returnvalue 0.7 :!class /Script/Engine.AudioComponent)
  (bind _returnvalue_2 (Game|SpawnActorfromClass "/Game/SideScrollerBP/Blueprints/Impulse_R.Impulse_R_C" (Math|Conversions|ToTransform(Vector) (Transformation|GetWorldLocation (Variables|Default|GetPaperSprite))) "Undefined" 0 0))
  (Transformation|SetActorScale3D _returnvalue_2 "1.800000,1.800000,1.800000")
  (Utilities|FlowControl|Delay 0.2)
  (Rendering|SetVisibility (Variables|Default|GetPaperSprite) true false)
  (Utilities|FlowControl|Delay 2.0)
  (bind _returnvalue_3 (Game|SpawnActorfromClass "/Game/SideScrollerBP/Blueprints/Impulse_R.Impulse_R_C" (Math|Conversions|ToTransform(Vector) (Transformation|GetWorldLocation (Variables|Default|GetPaperSprite))) "Undefined" 0 0))
  (Transformation|SetActorScale3D _returnvalue_3 "1.800000,1.800000,1.800000")
  (bind _returnvalue_4 (Audio|SpawnSound2D "/Game/Se/Flash2.Flash2" 1.0 1.0 0.0 0))
  (Audio|Components|Audio|SetPitchMultiplier _returnvalue_4 1.2)
  (Audio|Components|Audio|SetVolumeMultiplier _returnvalue_4 0.7 :!class /Script/Engine.AudioComponent)
  (Utilities|FlowControl|Delay 0.2)
  (Actor|DestroyActor))

(fn ConstructionScript)