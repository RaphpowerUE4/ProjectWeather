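; BP_Weather is a weather controller actor that turns storm, fog and frost intensity values into screen, camera and lighting effects.
; Every Tick it looks up the height fog and C_PostWeatherFX actors, setting second fog density, frost, screen drops and look intensity.
; It also starts a storm camera shake scaled by StormEffects each frame.
; A looping timer with random delays double-flashes a directional light as lightning while StormEffects is non-zero.
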(event Custom|LightingLoop
  (Utilities|FlowControl|Delay (Math|Random|RandomFloatinRange 5.0 2e+01))
  (if (not (Math|Float|NearlyEqual(Float) (Variables|Default|GetStormEffects) 0.0 1e-06))
    (CallFunction|LightingStrike)))

(event Custom|LightingStrike
  (Rendering|SetVisibility (Variables|Default|GetDirectionalLight) true false)
  (Utilities|FlowControl|Delay 0.05)
  (Rendering|SetVisibility (Variables|Default|GetDirectionalLight) false false)
  (Utilities|FlowControl|Delay 0.1)
  (Rendering|SetVisibility (Variables|Default|GetDirectionalLight) true false)
  (Utilities|FlowControl|Delay 0.06)
  (Rendering|SetVisibility (Variables|Default|GetDirectionalLight) false false))

(event EventTick
  (params (DeltaSeconds :type Float%20%28single-precision%29))
  (bind _stormeffects (Variables|Default|GetStormEffects))
  (bind _returnvalue (Actor|GetActorOfClass "/Script/Engine.ExponentialHeightFog"))
  (Variables|Default|SetFogVar _returnvalue)
  (bind _returnvalue_2 (Actor|GetActorOfClass "/Game/Chameleon/C_PostWeatherFX.C_PostWeatherFX_C"))
  (Variables|Default|SetPostFX _returnvalue_2)
  (Utilities|FlowControl|Sequence
    (:then_0
      (Variables|/Game/Chameleon/Chameleon.Chameleon_C|SetFrost%20-%20Advanced (Variables|Default|GetPostFX) (Utilities|Struct|MakeAdvancedEffectFeatures "NewEnumerator0" 0 "(X_2_61690A0C49AE65EEBEA3F1869ED7C8B0=1.000000,Y_4_99EA40724D71AB71DA2E298FBE765633=1.000000)" 0.0 1e+01 false (Variables|Default|GetFrostEffects) 0 false false false 0)))
    (:then_1
      (Class|ExponentialHeightFogComponent|SetSecondFogDensity (Variables|/Script/Engine.ExponentialHeightFog|GetComponent (Variables|Default|GetFogVar)) (Variables|Default|GetFogEffects)))
    (:then_2
      (CameraShakes|StartCameraShake (Game|GetPlayerCameraManager 0) "/Game/WTHR/Blueprints/Shakes/BP_StormShake.BP_StormShake_C" _stormeffects "CameraLocal" "0, 0, 0")
      (Variables|/Game/Chameleon/Chameleon.Chameleon_C|SetScreen%20Drops%20-%20Advanced (Variables|Default|GetPostFX) (Utilities|Struct|MakeAdvancedEffectFeatures "NewEnumerator0" 0 "(X_2_61690A0C49AE65EEBEA3F1869ED7C8B0=1.000000,Y_4_99EA40724D71AB71DA2E298FBE765633=1.000000)" 0.0 1e+01 false _stormeffects 0 false false false 0))
      (Variables|/Game/Chameleon/Chameleon.Chameleon_C|SetLOOK!%20Intensity (Variables|Default|GetPostFX) _stormeffects))))

(event EventBeginPlay
  (Utilities|Time|SetTimerbyEvent (delegate Custom|LightingLoop) 3.0 true))

(fn ConstructionScript)