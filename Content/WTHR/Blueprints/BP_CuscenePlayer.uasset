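; Cutscene player actor that spawns and plays a configured Level Sequence, either on BeginPlay or through LaunchSequencer.
; An existing sequence actor blocks relaunch; otherwise playback starts after a configurable delay, with play, finish and camera-cut callbacks bound.
; Player input is optionally disabled during playback.
; Restoring input and destroying the sequence actor require EndEvents, and each stage prints debug info to screen.
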(event Custom|LaunchSequencer
  (Utilities|IsValid (Variables|Private|GetRunningSequenceReference) ; Make sure we aren't playing sequence already
    (:Is%20Not%20Valid
      (bind _outactor (Sequencer|Player|CreateLevelSequencePlayer (Variables|Cutscene|GetSequenceToPlay) (Variables|Cutscene|GetSequenceSettings))) ; SetupLevelSequenceActor
      (Variables|Private|SetRunningSequenceReference _outactor)
      (CallFunction|BeforeSequenceStarts))))

(event Custom|OnSequencePlayEvents
  ;[0.06995 0.3927 0.0752] When sequence Starts
  (CallFunction|PrintSequenceInfo "Play Events Sucess")
  (if (Variables|Cutscene|GetDisablePlayerControl)
    (Input|DisableInput (Game|GetPlayerCharacter 0) (Game|GetPlayerController 0))))

(event Custom|BeforeSequenceStarts
  ;[0.3719 0.3024 0] Before sequence starts
  (CallFunction|PrintSequenceInfo "Before Play Events Sucess")
  (Utilities|FlowControl|Delay (Variables|Cutscene|GetDelayBeforeSequenceStart))
  (CallFunction|StartCreatedSequence))

(event Custom|StartCreatedSequence
  (bind _runningsequencereference (Variables|Private|GetRunningSequenceReference))
  (bind _sequenceplayer (Variables|/Script/LevelSequence.LevelSequenceActor|GetSequencePlayer _runningsequencereference))
  ;[0.02843 0.159 0.03071] Sequence actualy plays
  (EventDispatchers|BindEventtoOnPlay _sequenceplayer (delegate Custom|OnSequencePlayEvents))
  (EventDispatchers|AssignOnFinished _sequenceplayer (delegate Custom|OnSequenceFinished))
  (EventDispatchers|BindEventtoOnCameraCut _sequenceplayer (delegate Custom|OnCameraCut))
  (Sequencer|Player|Play _sequenceplayer :!class /Script/MovieScene.MovieSceneSequencePlayer))

(event Custom|OnSequenceFinished
  ;[0.5052 0 0.02479] When sequence finished playing
  (if (Variables|Cutscene|GetEndEvents)
    (CallFunction|PrintSequenceInfo "End Events Sucess")
    (if (Variables|Cutscene|GetDisablePlayerControl)
      (Input|EnableInput (Game|GetPlayerCharacter 0) (Game|GetPlayerController 0)))
    (Actor|DestroyActor (Variables|Private|GetRunningSequenceReference))
    (else
      (CallFunction|PrintSequenceInfo "End Events Disabled"))))

(event Custom|OnCameraCut
  (params (CameraComponent :type Camera%20Component%20Object%20Reference))
  ;[1 0.3538 0.2359] When a camera cut is detected inside the sequence
  (CallFunction|PrintSequenceInfo (Utilities|String|Append "Cut Detected = " (Utilities|GetDisplayName CameraComponent))))

(event EventBeginPlay
  (Variables|Default|SetTags (Variables|Tags|GetActorTag))
  (if (Variables|Cutscene|GetPlayAtBeginPlay)
    (CallFunction|LaunchSequencer)))

(fn ConstructionScript)

(fn PrintSequenceInfo
  (params (InfoToPrint :type String))
  (bind _runningsequencereference (Variables|Private|GetRunningSequenceReference))
  (Utilities|IsValid _runningsequencereference
    (:Is%20Valid
      (Development|PrintString (Utilities|String|Append "Sequence: " (Utilities|GetDisplayName (Class|LevelSequenceActor|GetSequence _runningsequencereference)) ": " InfoToPrint)))
    (:Is%20Not%20Valid
      (Development|PrintString (Utilities|String|Append "Sequence: " (Utilities|GetDisplayName self) ": " "[ERROR]: Couldn't Find Sequence (Sequence Invalid)") true true "(R=1.000000,G=0.000000,B=0.005232,A=1.000000)"))))